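; BP_PlayerCharactor01 is the side-scrolling player character, moving along the X axis with a flipped sprite, jumping and talking to the guide NPC.
; BeginPlay adds the Enhanced Input mapping context and base UI, and movement is gated by CanMove.
; Interact finds BP_NPC_Guide and shows its dialogue widget when PlayerInRange is set, otherwise removing it.
; AnyDamage subtracts from HP with no death handling here.
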(event Custom|SetUI_NPCGuide
  (bind _returnvalue (UserInterface|CreateWidget "/Game/NPCGuide/widget/UI_forNPCGuid.UI_forNPCGuid_C"))
  (Widget|SetVisibility (Variables|/Game/NPCGuide/widget/UI_forNPCGuid.UI_forNPCGuid_C|Gettxt_NPCtalk _returnvalue) "Visible")
  (UserInterface|Viewport|AddtoViewport _returnvalue 0))

(event Custom|set_uiNPCGuideRemove
  (Widget|RemovefromParent (stale Custom|SetUI_NPCGuide _returnvalue)))

(event Custom|SetUIBase
  (bind _returnvalue (UserInterface|CreateWidget "/Game/C03_01/UI_Base.UI_Base_C"))
  (UserInterface|Viewport|AddtoViewport _returnvalue 0))

(event Input|EnhancedActionEvents|EnhancedInputActionIA_Move01
  (params (ActionValue :type Float%20%28double-precision%29) (ElapsedSeconds :type Float%20%28double-precision%29) (TriggeredSeconds :type Float%20%28double-precision%29) (InputAction :type Input%20Action%20Object%20Reference :default "/Game/C03_01/Input/IA_Move01.IA_Move01"))
  (bind _returnvalue (Math|Conversions|ToVector2D(Vector) ActionValue))
  (bind _playersprite (Variables|Default|GetPlayerSprite))
  (bind _x (Math|Vector2D|BreakVector2D _returnvalue))
  (if (Variables|Default|GetCanMove)
    (if (> _x 0.0)
      (Variables|Default|SetIsFacingRight true)
      (else
        (Variables|Default|SetIsFacingRight false)))
    (Pawn|Input|AddMovementInput "1.000000,0.000000,0.000000" _x false)
    (if (Variables|Default|GetIsFacingRight)
      (Transformation|SetRelativeRotation _playersprite "0, 0, 0" false false)
      (else
        (Transformation|SetRelativeRotation _playersprite "0.000000,180.000000,0.000000" false false)))
    (else
      (Development|PrintString "Move Locked"))))

(event Input|EnhancedActionEvents|EnhancedInputActionIA_Jump01
  (params (ActionValue :type Boolean) (ElapsedSeconds :type Float%20%28double-precision%29) (TriggeredSeconds :type Float%20%28double-precision%29) (InputAction :type Input%20Action%20Object%20Reference :default "/Game/C03_01/Input/IA_Jump01.IA_Jump01"))
  (:Started
    (Character|Jump))
  (:Completed
    (Character|StopJumping)))

(event Input|EnhancedActionEvents|EnhancedInputActionIA_Interact
  (params (ActionValue :type Boolean) (ElapsedSeconds :type Float%20%28double-precision%29) (TriggeredSeconds :type Float%20%28double-precision%29) (InputAction :type Input%20Action%20Object%20Reference :default "/Game/C03_01/Input/IA_Interact.IA_Interact"))
  (:Started
    (bind _returnvalue (Actor|GetActorOfClass "/Game/NPCGuide/BP_NPC_Guide.BP_NPC_Guide_C"))
    (bind _asbp_npc_guide (Utilities|Casting|CastToBP_NPC_Guide _returnvalue))
    (if (Variables|/Game/NPCGuide/BP_NPC_Guide.BP_NPC_Guide_C|GetPlayerInRange _asbp_npc_guide)
      (CallFunction|SetUINPCGuide)
      (else
        (Development|PrintString "No NPC")
        (CallFunction|SetUiNPCGuideRemove)))))

(event EventBeginPlay
  (Input|AddMappingContext (PlayerController|LocalPlayerSubsystems|GetEnhancedInputLocalPlayerSubsystem (Game|GetPlayerController 0)) "/Game/C03_01/Input/IMC_Player01.IMC_Player01" 0 "(bIgnoreAllPressedKeysUntilRelease=True,bForceImmediately=False,bNotifyUserSettings=False)")
  (CallFunction|SetUIBase))

(event Collision|EventActorBeginOverlap
  (params (OtherActor :type Actor%20Object%20Reference)))

(event EventTick
  (params (DeltaSeconds :type Float%20%28single-precision%29)))

(event Game|Damage|EventAnyDamage
  (params (Damage :type Float%20%28single-precision%29) (DamageType :type Damage%20Type%20Object%20Reference) (InstigatedBy :type Controller%20Object%20Reference) (DamageCauser :type Actor%20Object%20Reference))
  (Variables|Default|SetHP (- (Variables|Default|GetHP) Damage)))

(fn ConstructionScript)