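; BP_ParallaxBackdrop is a backdrop actor that creates horizontal parallax between far and mid background layers as the player moves.
; It records the player character's starting X on BeginPlay, then calls UpdateParallax every Tick.
; UpdateParallax scales the player's X displacement by a separate factor per layer and sets SPFar and SPMid relative locations from shared start coordinates, with fixed Y offsets separating their depths.
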(event `self.ReceiveBeginPlay`
  (set `self.PlayerStartX` (.x (`self.K2_GetActorLocation` (`GameplayStatics.GetPlayerCharacter` 0)))))

(event `self.ReceiveTick`
  (params (DeltaSeconds :type "Float (single-precision)"))
  (`self.UpdateParallax`))

(fn `UpdateParallax`
  (set `self.DeltaX` (- (.x (`self.K2_GetActorLocation` (`GameplayStatics.GetPlayerCharacter` 0))) (`self.PlayerStartX`)))
  (`|ExecutionSequence`
    (:`then_0`
      (`SceneComponent.K2_SetRelativeLocation` (`self.SP_Far`) (`KismetMathLibrary.MakeVector` (+ (`self.XStart`) (* (`self.DeltaX`) (`self.FarGB`))) (+ (`self.YStart`) -200.0) (`self.ZStart`)) false false))
    (:`then_1`
      (`SceneComponent.K2_SetRelativeLocation` (`self.SP_Mid`) (`KismetMathLibrary.MakeVector` (+ (`self.XStart`) (* (`self.DeltaX`) (`self.MidGB`))) (+ (`self.YStart`) -100.0) (`self.ZStart`)) false false))))

(fn `UserConstructionScript`)